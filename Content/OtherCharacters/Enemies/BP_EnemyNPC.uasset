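; Enemy NPC Blueprint that detects the main character through PawnSensing and feeds that state to its AI Blackboard.
; A sighting stores the player and their last location, sets the visibility flags and switches movement to sprint speed.
; Two chained timelines act as timers restarted by sightings: CheckPlayer clears CanSeePlayer, then ForgetPlayer, sized from Stats, marks the player lost and restores walk speed.
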(event `self.ReceiveBeginPlay`
  (bind (_stats_sprintspeed _stats_walkspeed _stats_accelerationspeed _stats_traction _stats_handling _stats_normalheight _stats_turnspeed _stats_forgettimer) (break `NPCStruct` (`self.stats`)))
  (set `self.playerLost` true)
  (set `CharacterMovementComponent.MaxWalkSpeed` _stats_walkspeed (`self.CharacterMovement`))
  (`TimelineComponent.SetTimelineLength` (`self.ForgetPlayerTimeline`) _stats_forgettimer))

(event `self.PawnSensing.OnSeePawn`
  (params (Pawn :type "Pawn Object Reference"))
  (bind _returnvalue (`AIBlueprintHelperLibrary.GetBlackboard` null))
  (bind (_stats_sprintspeed _stats_walkspeed _stats_accelerationspeed _stats_traction _stats_handling _stats_normalheight _stats_turnspeed _stats_forgettimer) (break `NPCStruct` (`self.stats`)))
  (if (`KismetMathLibrary.ClassIsChildOf` (`GameplayStatics.GetObjectClass` Pawn) "/Game/MainCharacterAssets/BP_MainCharacter.BP_MainCharacter_C")
    (`BlackboardComponent.SetValueAsObject` _returnvalue "PlayerObj" Pawn)
    (`BlackboardComponent.SetValueAsVector` _returnvalue "LastPlayerLocation" (`self.K2_GetActorLocation` Pawn))
    (bind _output_get (set `CharacterMovementComponent.MaxWalkSpeed` _stats_sprintspeed (`self.CharacterMovement`)))
    (`KismetSystemLibrary.PrintString` (`KismetStringLibrary.Conv_DoubleToString` _output_get))
    (bind _output_get_2 (set `self.playerLost` false))
    (bind _output_get_3 (set `self.canSeePlayer` true))
    (`BlackboardComponent.SetValueAsBool` _returnvalue "PlayerLost" _output_get_2)
    (`BlackboardComponent.SetValueAsBool` _returnvalue "CanSeePlayer" _output_get_3)
    (`Timeline|CheckPlayerTimeline` :!via `PlayFromStart`
      (:`Finished`
        (bind _output_get_4 (set `self.canSeePlayer` false))
        (`BlackboardComponent.SetValueAsBool` _returnvalue "CanSeePlayer" _output_get_4)
        (`Timeline|ForgetPlayerTimeline` :!via `PlayFromStart`
          (:`Finished`
            (bind _output_get_5 (set `self.playerLost` true))
            (set `CharacterMovementComponent.MaxWalkSpeed` _stats_walkspeed (`self.CharacterMovement`))
            (`BlackboardComponent.SetValueAsBool` _returnvalue "PlayerLost" _output_get_5)))))))

(fn `UserConstructionScript`)