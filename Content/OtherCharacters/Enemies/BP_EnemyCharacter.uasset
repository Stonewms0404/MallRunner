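; Enemy character that detects the player through pawn sensing and chooses patrol locations.
; Sightings switch it to sprint and write the player and last known location to the Blackboard.
; Chained timers clear visibility shortly after a sighting, then mark the player lost and restore walk speed after a forget delay.
; Patrol selection samples random pedestrian positions against a distance threshold, or random coordinates when none exist.
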(event `self.ReceiveBeginPlay`
  (set `self.playerLost` true))

(event `LostPlayer`
  (bind (_stats_sprintspeed _stats_walkspeed _stats_accelerationspeed _stats_traction _stats_handling _stats_normalheight _stats_turnspeed _stats_forgettimer) (break `NPCStruct` (`self.stats`)))
  (set `self.playerLost` true)
  (set `CharacterMovementComponent.MaxWalkSpeed` _stats_walkspeed (`self.CharacterMovement`)))

(event `Can'tSeePlayer`
  (bind (_stats_sprintspeed _stats_walkspeed _stats_accelerationspeed _stats_traction _stats_handling _stats_normalheight _stats_turnspeed _stats_forgettimer) (break `NPCStruct` (`self.stats`)))
  (set `self.canSeePlayer` false)
  (`KismetSystemLibrary.K2_SetTimerDelegate` (delegate `LostPlayer`) _stats_forgettimer))

(event `self.PawnSensing.OnSeePawn`
  (params (Pawn :type "Pawn Object Reference"))
  (bind _returnvalue (`AIBlueprintHelperLibrary.GetBlackboard` null))
  (bind (_stats_sprintspeed _stats_walkspeed _stats_accelerationspeed _stats_traction _stats_handling _stats_normalheight _stats_turnspeed _stats_forgettimer) (break `NPCStruct` (`self.stats`)))
  (bind _asbp_main_character (cast `/Game/MainCharacterAssets/BP_MainCharacter` Pawn))
  (set `CharacterMovementComponent.MaxWalkSpeed` _stats_sprintspeed (`self.CharacterMovement`))
  (set `self.canSeePlayer` true)
  (set `self.playerLost` false)
  (`BlackboardComponent.SetValueAsVector` _returnvalue "LastPlayerLocation" (`self.K2_GetActorLocation` _asbp_main_character))
  (`BlackboardComponent.SetValueAsObject` _returnvalue "PlayerObj" _asbp_main_character)
  (`KismetSystemLibrary.K2_SetTimerDelegate` (delegate `Can'tSeePlayer`) 0.5))

(event `self.GetSetPatrolLocation`
  (bind _returnvalue (`self.K2_GetActorLocation`))
  (bind _outactors (`GameplayStatics.GetAllActorsOfClass` "/Game/OtherCharacters/Pedestrians/BP_PedestrianCharacter.BP_PedestrianCharacter_C"))
  (if (== (`KismetArrayLibrary.Array_Length` _outactors) 0)
    (set `self.patrolLocation` (`KismetMathLibrary.MakeVector` (`KismetMathLibrary.Conv_IntToDouble` (`KismetMathLibrary.RandomInteger` 500)) (`KismetMathLibrary.Conv_IntToDouble` (`KismetMathLibrary.RandomInteger` 500)) (.z _returnvalue)))
    (else
      (bind _returnvalue_2 (`self.K2_GetActorLocation` (`KismetArrayLibrary.Array_Random` _outactors)))
      (while (< (`KismetMathLibrary.VSize` (- _returnvalue_2 _returnvalue)) 3000.0)
        (set `self.patrolLocation` _returnvalue_2)))))

(fn `UserConstructionScript`)