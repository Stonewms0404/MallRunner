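; Player character Blueprint that sets up Enhanced Input and handles crouch and slide transitions.
; BeginPlay adds the main mapping context through the MainPlayerController.
; A reversible timeline blends capsule half-height for crouching, while another blends max walk speed from slide to crouch speed.
; Cancelling a slide applies the supplied speed immediately and holds it on timeline updates until the timeline finishes and re-enables sliding.
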(event `self.ReceiveBeginPlay`
  (bind _asmain_player_controller (cast `MainPlayerController` (`self.GetController`)))
  (bind _returnvalue (pcsubsystem `EnhancedInputLocalPlayerSubsystem` _asmain_player_controller))
  (`/Engine/EditorBlueprintResources/StandardMacros.IsValid` _returnvalue
    (:`Is Valid`
      (`EnhancedInputSubsystemInterface.AddMappingContext` _returnvalue "/Game/Input/IA_Main_Mapping.IA_Main_Mapping" 0 (struct)))))

(event `self.OnCrouchChanged`
  (params (Crouching :type Boolean))
  (if Crouching
    (bind (_direction _crouch) (`Timeline|Timeline_Crouch` :!via `Reverse` :!label _label)
      (:`Update`
        (`CapsuleComponent.SetCapsuleHalfHeight` (`self.CapsuleComponent`) (`KismetMathLibrary.Lerp` 88.0 40.0 _crouch) true)))
    (else
      (goto _label))))

(event `self.OnPlayerSlide`
  (params (SlideSpeed :type "Float (single-precision)") (CrouchSpeed :type "Float (single-precision)"))
  (bind _charactermovement (`self.CharacterMovement`))
  (bind (_direction _crouch) (`Timeline|Timeline` :!via `PlayFromStart`)
    (:`Update`
      (if (`self.CanSlide`)
        (set `CharacterMovementComponent.MaxWalkSpeed` (`KismetMathLibrary.Lerp` SlideSpeed CrouchSpeed _crouch) _charactermovement)
        (else
          (set `CharacterMovementComponent.MaxWalkSpeed` (stale `self.OnCancelSlide` _output_get) _charactermovement :!label _label_2))))
    (:`Finished`
      (set `self.CanSlide` true))))

(event `self.OnCancelSlide`
  (params (cancel :type Boolean) (Speed :type "Float (single-precision)"))
  (set `self.CanSlide` false)
  (bind _output_get (set `self.SprintSpeed` Speed))
  (goto _label_2))

(fn `UserConstructionScript`)